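; BP_Quest is the base Blueprint for quests in the objective system, holding a root objective collection.
; On BeginPlay it constructs the root collection, passes it to PopulateObjectives to be filled, then activates it.
; Construction and population are template steps for child quests to override; the base versions only print red error messages.
; A getter exposes the root collection to other code.
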(event `self.ReceiveBeginPlay`
  (bind _rootobjcollection (`self.ConstructRootObjectiveCollection`))
  (bind _output_get (set `self.RootObjectiveCollection` _rootobjcollection))
  (`self.PopulateObjectives` _output_get)
  (`/Game/ObjectiveSystem/Objectives/BP_Objective.ActivateObjective` (`self.RootObjectiveCollection`)))

(fn `ConstructRootObjectiveCollection`
  (returns (RootObjCollection :type "/Game/ObjectiveSystem/Objectives/BP_ObjCollection Object Reference"))
  (`KismetSystemLibrary.PrintString` "Error: CreateRootObjectiveCollection called for base class!" true true (struct :`R` 1.0 :`A` 1.0))
  (return null))

(fn `GetRootObjectiveCollection`
  (returns (RootObjectiveCollection :type "/Game/ObjectiveSystem/Objectives/BP_ObjCollection Object Reference"))
  (return (`self.RootObjectiveCollection`)))

(fn `PopulateObjectives`
  (params (RootObjCollection :type "/Game/ObjectiveSystem/Objectives/BP_ObjCollection Object Reference"))
  (`KismetSystemLibrary.PrintString` "Error: PopulateObjectives called for base class!" true true (struct :`R` 1.0 :`A` 1.0)))

(fn `UserConstructionScript`)