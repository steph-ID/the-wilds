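; BP_Obj_PickUpItem is an objective that completes when the player picks up a designated item.
; On activation it runs the parent logic and binds to the PickupItem actor's begin-overlap event.
; When the player character overlaps the item, it unbinds, sets ItemCollected and fires OnCompleted.
; GetIsComplete reports the ItemCollected flag.
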(event `self.ActivateObjective`
  (`parent.ActivateObjective`)
  (add `Actor.OnActorBeginOverlap` (`self.PickupItem`) (delegate `OnActorBeginOverlap_Event`)))

(event `OnActorBeginOverlap_Event`
  (params (OverlappedActor :type "Actor Object Reference") (OtherActor :type "Actor Object Reference"))
  (cast `/Game/Actors/Player/BP_PlayerCharacter` OtherActor)
  (remove `Actor.OnActorBeginOverlap` (`self.PickupItem`) (delegate `OnActorBeginOverlap_Event`))
  (set `self.ItemCollected` true)
  (`self.OnCompleted` self))

(fn `GetIsComplete`
  (returns (IsComplete :type Boolean))
  (return (`self.ItemCollected`)))