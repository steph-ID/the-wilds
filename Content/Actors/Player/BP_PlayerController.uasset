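; Player controller that handles the player's shooting, sprinting and menu input through Enhanced Input actions.
; On BeginPlay it caches the character's default walk speed and gathers all BP_Quest actors into Quests.
; Sprint multiplies that walk speed while active and restores it on completion, and shooting spawns BP_Projectile at the pawn's location with a slight offset.
; Objectives and in-game menu inputs each create a new widget, add it to the viewport and focus it.
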(event `self.ReceiveBeginPlay`
  (bind _asbp_player_character (cast `/Game/Actors/Player/BP_PlayerCharacter` (`self.K2_GetPawn`)))
  (set `self.DefaultWalkSpeed` (`CharacterMovementComponent.MaxWalkSpeed` (`Character.CharacterMovement` _asbp_player_character)))
  (bind _outactors (`GameplayStatics.GetAllActorsOfClass` "/Game/ObjectiveSystem/Quests/BP_Quest.BP_Quest_C"))
  (set `self.Quests` _outactors))

(event `EnhancedInput|/Game/Actors/Player/Actions/IA_Shoot`
  (params (ActionValue :type Boolean) (ElapsedSeconds :type "Float (double-precision)") (TriggeredSeconds :type "Float (double-precision)") (InputAction :type "InputAction Object Reference" :default "/Game/Actors/Player/Actions/IA_Shoot.IA_Shoot"))
  (:`Triggered`
    (`|SpawnActorFromClass` "/Game/BP_Projectile.BP_Projectile_C" (`KismetMathLibrary.MakeTransform` (+ (`self.K2_GetActorLocation` (`self.K2_GetPawn`)) (0.2 0.0 0.0))) "AdjustIfPossibleButAlwaysSpawn" "OverrideRootScale" null null)))

(event `EnhancedInput|/Game/Actors/Player/Actions/IA_Sprint`
  (params (ActionValue :type Boolean) (ElapsedSeconds :type "Float (double-precision)") (TriggeredSeconds :type "Float (double-precision)") (InputAction :type "InputAction Object Reference" :default "/Game/Actors/Player/Actions/IA_Sprint.IA_Sprint"))
  (bind _returnvalue (`self.K2_GetPawn`))
  (bind _defaultwalkspeed (`self.DefaultWalkSpeed`))
  (:`Triggered`
    (bind _asbp_player_character (cast `/Game/Actors/Player/BP_PlayerCharacter` _returnvalue))
    (set `CharacterMovementComponent.MaxWalkSpeed` (* _defaultwalkspeed (`self.SprintMultiplier`)) (`Character.CharacterMovement` _asbp_player_character)))
  (:`Completed`
    (bind _asbp_player_character_2 (cast `/Game/Actors/Player/BP_PlayerCharacter` _returnvalue))
    (set `CharacterMovementComponent.MaxWalkSpeed` _defaultwalkspeed (`Character.CharacterMovement` _asbp_player_character_2))))

(event `EnhancedInput|/Game/Actors/Player/Actions/IA_OpenObjectives`
  (params (ActionValue :type Boolean) (ElapsedSeconds :type "Float (double-precision)") (TriggeredSeconds :type "Float (double-precision)") (InputAction :type "InputAction Object Reference" :default "/Game/Actors/Player/Actions/IA_OpenObjectives.IA_OpenObjectives"))
  (:`Triggered`
    (bind _returnvalue (`|CreateWidget` "/Game/ObjectiveSystem/UI/WBP_Objectives.WBP_Objectives_C" (`GameplayStatics.GetPlayerController` 0)))
    (`UserWidget.AddToViewport` _returnvalue 0)
    (`Widget.SetFocus` _returnvalue)))

(event `EnhancedInput|/Game/Actors/Player/Actions/IA_Menu`
  (params (ActionValue :type Boolean) (ElapsedSeconds :type "Float (double-precision)") (TriggeredSeconds :type "Float (double-precision)") (InputAction :type "InputAction Object Reference" :default "/Game/Actors/Player/Actions/IA_Menu.IA_Menu"))
  (:`Triggered`
    (bind _returnvalue (`|CreateWidget` "/Game/UI/WBP_InGameMenu.WBP_InGameMenu_C" (`GameplayStatics.GetPlayerController` 0)))
    (bind _output_get (set `self.Menu` _returnvalue))
    (`UserWidget.AddToViewport` _output_get 0)
    (`UserWidget.AddToViewport` _returnvalue 0)
    (`Widget.SetFocus` (`self.Menu`))))

(fn `UserConstructionScript`)