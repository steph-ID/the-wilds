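; BP_Quest_01 is a quest definition in the objective system that sends the player through an ordered series of waypoint objectives.
; It builds a root BP_ObjCollection with order enforcement enabled, named from the quest's objective name.
; PopulateObjectives adds three BP_Obj_ReachWaypoint objectives to it: jumping a rock, crossing a bridge and recovering health.
; An unconnected pick-up-item version of the health objective never runs, and the event graph is inactive.
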(fn `ConstructRootObjectiveCollection`
  (returns (RootObjCollection :type "/Game/ObjectiveSystem/Objectives/BP_ObjCollection Object Reference"))
  (bind _returnvalue (`|GenericCreateObject` "/Game/ObjectiveSystem/Objectives/BP_ObjCollection.BP_ObjCollection_C" true (`self.ObjectiveName`)))
  (return _returnvalue))

(fn `PopulateObjectives`
  (params (RootObjCollection :type "/Game/ObjectiveSystem/Objectives/BP_ObjCollection Object Reference"))
  (`|ExecutionSequence`
    (:`then_0`
      (bind _returnvalue (`|GenericCreateObject` "/Game/ObjectiveSystem/Objectives/BP_Obj_ReachWaypoint.BP_Obj_ReachWaypoint_C" (`self.RockWaypoint`) "Jump over the rock"))
      (`/Game/ObjectiveSystem/Objectives/BP_ObjCollection.AddObjective` (`local.RootObjCollection`) _returnvalue))
    (:`then_1`
      (bind _returnvalue_2 (`|GenericCreateObject` "/Game/ObjectiveSystem/Objectives/BP_Obj_ReachWaypoint.BP_Obj_ReachWaypoint_C" (`self.BridgeWaypoint`) "Cross the bridge"))
      (`/Game/ObjectiveSystem/Objectives/BP_ObjCollection.AddObjective` (`local.RootObjCollection`) _returnvalue_2))
    (:`then_2`
      (bind _returnvalue_3 (`|GenericCreateObject` "/Game/ObjectiveSystem/Objectives/BP_Obj_ReachWaypoint.BP_Obj_ReachWaypoint_C" (`self.HealthWaypoint`) "Recover your health"))
      (`/Game/ObjectiveSystem/Objectives/BP_ObjCollection.AddObjective` (`local.RootObjCollection`) _returnvalue_3))))

(fn `UserConstructionScript`
  (`parent.UserConstructionScript`))